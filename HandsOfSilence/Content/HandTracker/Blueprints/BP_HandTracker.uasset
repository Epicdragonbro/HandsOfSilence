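; BP_HandTracker tracks left and right hands in a playing video through a MediaPipe component and raises hand-tracking and pinch events.
; Each tick it draws the video material to a render target for landmark detection and matches camera and tracker FOV to video and viewport aspect.
; Palm position averages seven landmarks; a pinch is thumb-to-index distance under a third of palm size.
; It also draws debug skeletons, optionally mirrored in editor.
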(event `Init`
  (`MediaPipeHandTrackerComponent.InitGraph` (`self.MediaPipeHandTracker`))
  (set `self.bInitialized` true))

(event `Shutdown`
  (if (`self.bInitialized`)
    (`MediaPipeHandTrackerComponent.ShutdownGraph` (`self.MediaPipeHandTracker`))
    (set `self.bInitialized` false)))

(event `self.ReceiveEndPlay`
  (params (EndPlayReason :type "EEndPlayReason Enum" :default "Destroyed"))
  (`self.Shutdown`))

(event `self.ReceiveTick`
  (params (DeltaSeconds :type "Float (single-precision)"))
  (bind _rendertargettexture (`self.RenderTargetTexture`))
  (if (`self.bInitialized`)
    (`|ExecutionSequence`
      (:`then_0`
        (if (`MediaPlayer.IsPlaying` (`self.MediaPlayer`))
          ;[1 1 1] Calculate Horizontal FOV for the Hand tracker component
          (`MediaPipeHandTrackerComponent.SetHFoV` (`self.MediaPipeHandTracker`) (* (`KismetMathLibrary.DegAtan` (* (/ (`KismetMathLibrary.Conv_IntToDouble` (`TextureRenderTarget2D.SizeX` _rendertargettexture)) (`KismetMathLibrary.Conv_IntToDouble` (`TextureRenderTarget2D.SizeY` _rendertargettexture))) (`KismetMathLibrary.DegTan` (/ (`self.DefaultCameraFOVVertical`) 2.0)))) 2.0))))
      (:`then_1`
        ;[1 1 1] Render target - Resizes the input video to 720p -> faster processing
        (`/Engine/EditorBlueprintResources/StandardMacros.IsValid` (`self.RenderTargetTexture`)
          (:`Is Valid`
            (`KismetRenderingLibrary.DrawMaterialToRenderTarget` (`self.RenderTargetTexture`) (`self.VideoMaterial`))
            (`MediaPipeHandTrackerComponent.GetHandLandmarksFromRenderTarget2D` (`self.MediaPipeHandTracker`) (`self.RenderTargetTexture`))
            (if (`MediaPlayer.IsPlaying` (`self.MediaPlayer`))
              (`self.Process Hands`)))))
      (:`then_3`
        (if (`MediaPlayer.IsPlaying` (`self.MediaPlayer`))
          (`self.UpdateCameraFov`))))))

(fn `ColorByValue`
  (params (Value :type "Float (double-precision)"))
  (returns (Color :type "LinearColor Structure"))
  (if (< Value 0.5)
    (return (struct :`R` 1.0 :`A` 1.0))
    (elif (>= Value 0.75)
      (return (struct :`G` 1.0 :`A` 1.0))
      (else
        (return (struct :`R` 1.0 :`G` 0.201022 :`A` 1.0))))))

(fn `Detect Pinch`
  (params (Hand :type Integer))
  (returns (bPinch :type Boolean))
  (bind _mediapipehandtracker (`self.MediaPipeHandTracker`))
  (bind _mediapipehandtracker_2 (`self.MediaPipeHandTracker`))
  (return (< (`KismetMathLibrary.VSize` (- (`MediaPipeHandTrackerComponent.GetLandmarkPosition` _mediapipehandtracker_2 Hand 4 true) (`MediaPipeHandTrackerComponent.GetLandmarkPosition` _mediapipehandtracker_2 Hand 8 true))) (/ (`KismetMathLibrary.VSize` (- (`MediaPipeHandTrackerComponent.GetLandmarkPosition` _mediapipehandtracker Hand 0 true) (`MediaPipeHandTrackerComponent.GetLandmarkPosition` _mediapipehandtracker Hand 17 true))) 3.0))))

(fn `DrawDebugBone`
  (params (`Landmark ID start` :type Integer) (`Landmark ID end` :type Integer) (Hand :type Integer) (Color :type "LinearColor Structure"))
  (bind _mediapipehandtracker (`self.MediaPipeHandTracker`))
  (bind _returnvalue (`MediaPipeHandTrackerComponent.GetLandmarkPosition` _mediapipehandtracker Hand `Landmark ID end` false))
  (bind _returnvalue_2 (`MediaPipeHandTrackerComponent.GetLandmarkPosition` _mediapipehandtracker Hand `Landmark ID start` false))
  (if (and (`MediaPipeHandTrackerComponent.IsWithEditor` (`self.MediaPipeHandTracker`)) (`self.bMirrored`))
    (`MediaPipeHandTrackerComponent.DrawLine` (`self.MediaPipeHandTracker`) (* _returnvalue_2 (-1.0 1.0 1.0)) (* _returnvalue (-1.0 1.0 1.0)) Color 0 1.0 0.0)
    (else
      (`MediaPipeHandTrackerComponent.DrawLine` (`self.MediaPipeHandTracker`) _returnvalue_2 _returnvalue Color 0 1.0 0.0))))

(fn `DrawDebugHand`
  (params (Color :type "LinearColor Structure") (Hand :type Integer) (Text :type String))
  (locals (HandId :type Integer) (ColorId :type "LinearColor Structure"))
  (bind _handid (`local.HandId`))
  (bind _colorid (`local.ColorId`))
  (bind _colorid_2 (`local.ColorId`))
  (bind _colorid_3 (`local.ColorId`))
  (bind _colorid_4 (`local.ColorId`))
  (bind _colorid_5 (`local.ColorId`))
  (bind _colorid_6 (`local.ColorId`))
  (bind _handid_2 (`local.HandId`))
  (bind _handid_3 (`local.HandId`))
  (bind _handid_4 (`local.HandId`))
  (bind _handid_5 (`local.HandId`))
  (bind _handid_6 (`local.HandId`))
  (set `local.HandId` Hand)
  (set `local.ColorId` Color)
  (for _index (range 21)
    (if (and (`MediaPipeHandTrackerComponent.IsWithEditor` (`self.MediaPipeHandTracker`)) (`self.bMirrored`))
      (bind _returnvalue (`MediaPipeHandTrackerComponent.GetLandmarkPosition` (`self.MediaPipeHandTracker`) Hand _index false))
      (`MediaPipeHandTrackerComponent.DrawPoint` (`self.MediaPipeHandTracker`) (* _returnvalue (-1.0 1.0 1.0)) Color 20.0 0 0.0)
      (else
        (`MediaPipeHandTrackerComponent.DrawPoint` (`self.MediaPipeHandTracker`) _returnvalue Color 20.0 0 0.0))))
  (`|ExecutionSequence`
    (:`then_0`
      (`self.DrawDebugBone` 0 1 _handid_2 _colorid_2)
      (`self.DrawDebugBone` 1 2 _handid_2 _colorid_2)
      (`self.DrawDebugBone` 2 3 _handid_2 _colorid_2)
      (`self.DrawDebugBone` 3 4 _handid_2 _colorid_2))
    (:`then_1`
      (`self.DrawDebugBone` 5 6 _handid_5 _colorid_3)
      (`self.DrawDebugBone` 6 7 _handid_5 _colorid_3)
      (`self.DrawDebugBone` 7 8 _handid_5 _colorid_3))
    (:`then_2`
      (`self.DrawDebugBone` 9 10 _handid_3 _colorid_4)
      (`self.DrawDebugBone` 10 11 _handid_3 _colorid_4)
      (`self.DrawDebugBone` 11 12 _handid_3 _colorid_4))
    (:`then_3`
      (`self.DrawDebugBone` 13 14 _handid_4 _colorid_5)
      (`self.DrawDebugBone` 14 15 _handid_4 _colorid_5)
      (`self.DrawDebugBone` 15 16 _handid_4 _colorid_5))
    (:`then_4`
      (`self.DrawDebugBone` 17 18 _handid_6 _colorid_6)
      (`self.DrawDebugBone` 18 19 _handid_6 _colorid_6)
      (`self.DrawDebugBone` 19 20 _handid_6 _colorid_6))
    (:`then_5`
      (`self.DrawDebugBone` 2 5 _handid _colorid)
      (`self.DrawDebugBone` 5 9 _handid _colorid)
      (`self.DrawDebugBone` 9 13 _handid _colorid)
      (`self.DrawDebugBone` 13 17 _handid _colorid)
      (`self.DrawDebugBone` 17 0 _handid _colorid))))

(fn `GetHandPosition`
  (params (Hand :type Integer))
  (returns (Position :type "Vector Structure"))
  (bind _mediapipehandtracker (`self.MediaPipeHandTracker`))
  (return (`KismetMathLibrary.GetVectorArrayAverage` (`|MakeArray` (`MediaPipeHandTrackerComponent.GetLandmarkPosition` _mediapipehandtracker Hand 0 false) (`MediaPipeHandTrackerComponent.GetLandmarkPosition` _mediapipehandtracker Hand 1 false) (`MediaPipeHandTrackerComponent.GetLandmarkPosition` _mediapipehandtracker Hand 2 false) (`MediaPipeHandTrackerComponent.GetLandmarkPosition` _mediapipehandtracker Hand 5 false) (`MediaPipeHandTrackerComponent.GetLandmarkPosition` _mediapipehandtracker Hand 9 false) (`MediaPipeHandTrackerComponent.GetLandmarkPosition` _mediapipehandtracker Hand 13 false) (`MediaPipeHandTrackerComponent.GetLandmarkPosition` _mediapipehandtracker Hand 17 false)))))

(fn `GetHandScale`
  (params (Hand :type Integer))
  (returns (Scale :type "Float (double-precision)"))
  (bind _mediapipehandtracker (`self.MediaPipeHandTracker`))
  (return (/ (`KismetMathLibrary.VSize` (- (`MediaPipeHandTrackerComponent.GetLandmarkPosition` _mediapipehandtracker Hand 0 true) (`MediaPipeHandTrackerComponent.GetLandmarkPosition` _mediapipehandtracker Hand 17 true))) 100.0)))

(fn `Process Hands`
  (locals (LeftHandId :type Integer) (RightHandId :type Integer))
  (bind _position (`self.GetHandPosition` (`local.RightHandId`)))
  (bind _returnvalue (`MediaPipeHandTrackerComponent.GetHandedness` (`self.MediaPipeHandTracker`) 1))
  (bind _returnvalue_2 (`MediaPipeHandTrackerComponent.GetHandedness` (`self.MediaPipeHandTracker`) 0))
  (bind _position_2 (`self.GetHandPosition` (`local.LeftHandId`)))
  (bind _position_3 (`self.GetHandPosition` (`local.RightHandId`)))
  (bind _position_4 (`self.GetHandPosition` (`local.LeftHandId`)))
  (`|ExecutionSequence`
    (:`then_0`
      (if (`KismetStringLibrary.EqualEqual_StrStr` _returnvalue_2 "Left")
        (set `local.LeftHandId` 0)
        (`/Engine/EditorBlueprintResources/StandardMacros.DoOnce` false :!label _label
          (:`Completed`
            (`KismetSystemLibrary.PrintString` "Left hand is tracking" true false (struct :`G` 0.66 :`B` 1.0 :`A` 1.0) 0.0)
            (bind _bpinch (`self.Detect Pinch` (`local.LeftHandId`)))
            (`|ExecutionSequence`
              (:`then_0`
                (`self.OnHandIsTracking` "Left" _position_2))
              (:`then_1`
                (`self.OnPinchDetected` "Left" _position_2 _bpinch))
              (:`then_2`
                (`self.DrawDebugHand` (`KismetMathLibrary.SelectColor` (struct :`R` 1.0 :`A` 1.0) (struct :`G` 0.371238 :`B` 0.55834 :`A` 1.0) _bpinch) (`local.LeftHandId`) "Left")))))
        (elif (`KismetStringLibrary.EqualEqual_StrStr` _returnvalue_2 "Right")
          (set `local.RightHandId` 0)
          (`/Engine/EditorBlueprintResources/StandardMacros.DoOnce` false :!label _label_2
            (:`Completed`
              (`KismetSystemLibrary.PrintString` "Right hand is tracking" true false (struct :`R` 1.0 :`G` 0.846693 :`A` 1.0) 0.0)
              (bind _bpinch_2 (`self.Detect Pinch` (`local.RightHandId`)))
              (`|ExecutionSequence`
                (:`then_0`
                  (`self.OnHandIsTracking` "Right" _position))
                (:`then_1`
                  (`self.OnPinchDetected` "Right" _position _bpinch_2))
                (:`then_2`
                  (`self.DrawDebugHand` (`KismetMathLibrary.SelectColor` (struct :`R` 1.0 :`A` 1.0) (struct :`R` 1.0 :`G` 0.846873 :`A` 1.0) _bpinch_2) (`local.RightHandId`) "Right"))))))))
    (:`then_1`
      (if (`KismetStringLibrary.EqualEqual_StrStr` _returnvalue "Left")
        (set `local.LeftHandId` 1)
        (goto _label)
        (elif (`KismetStringLibrary.EqualEqual_StrStr` _returnvalue "Right")
          (set `local.RightHandId` 1)
          (goto _label_2))))
    (:`then_2`
      (goto _label :!via `Reset`))
    (:`then_3`
      (goto _label_2 :!via `Reset`))
    (:`then_4`
      ;[1 1 1] Palm positions
      (if (and (`MediaPipeHandTrackerComponent.IsWithEditor` (`self.MediaPipeHandTracker`)) (`self.bMirrored`))
        (`MediaPipeHandTrackerComponent.DrawPoint` (`self.MediaPipeHandTracker`) (* _position_4 (-1.0 1.0 1.0)) (struct :`G` 1.0 :`A` 1.0) 20.0 0 0.0)
        (`MediaPipeHandTrackerComponent.DrawPoint` (`self.MediaPipeHandTracker`) (* _position_3 (-1.0 1.0 1.0)) (struct :`G` 1.0 :`A` 1.0) 20.0 0 0.0)
        (else
          (`MediaPipeHandTrackerComponent.DrawPoint` (`self.MediaPipeHandTracker`) _position_4 (struct :`G` 1.0 :`A` 1.0) 20.0 0 0.0)
          (`MediaPipeHandTrackerComponent.DrawPoint` (`self.MediaPipeHandTracker`) _position_3 (struct :`G` 1.0 :`A` 1.0) 20.0 0 0.0))))))

(fn `UpdateCameraFov`
  (bind _defaultcamerafovvertical (`self.DefaultCameraFOVVertical`))
  (bind _rendertargettexture (`self.RenderTargetTexture`))
  (bind (_sizex _sizey) (`PlayerController.GetViewportSize` (`GameplayStatics.GetPlayerController` 0)))
  (bind _cameracomponent (`CameraActor.CameraComponent` (`self.Camera`)))
  (bind _returnvalue (/ (`KismetMathLibrary.Conv_IntToDouble` (`TextureRenderTarget2D.SizeX` _rendertargettexture)) (`KismetMathLibrary.Conv_IntToDouble` (`TextureRenderTarget2D.SizeY` _rendertargettexture))))
  (bind _returnvalue_2 (/ (`KismetMathLibrary.Conv_IntToDouble` _sizex) (`KismetMathLibrary.Conv_IntToDouble` _sizey)))
  ;[1 1 1] Camera FOV
  (bind _output_get (set `CameraComponent.AspectRatio` _returnvalue_2 (`CameraActor.CameraComponent` (`self.Camera`))))
  (if (>= _returnvalue _output_get)
    (set `CameraComponent.FieldOfView` (* (`KismetMathLibrary.DegAtan` (* _returnvalue_2 (`KismetMathLibrary.DegTan` (/ _defaultcamerafovvertical 2.0)))) 2.0) _cameracomponent)
    (else
      (set `CameraComponent.FieldOfView` (* (`KismetMathLibrary.DegAtan` (* _returnvalue (`KismetMathLibrary.DegTan` (/ _defaultcamerafovvertical 2.0)))) 2.0) _cameracomponent))))

(fn `UserConstructionScript`)