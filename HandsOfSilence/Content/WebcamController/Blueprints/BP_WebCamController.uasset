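; Webcam controller that creates a selector UI for picking a capture device, track, resolution and frame rate, then starts or stops Media Player playback.
; Each dropdown selection cascades into the next, favouring preferred resolution and FPS, until the matching track format is applied and Start is enabled.
; Short delays space out the Media Player and UI steps.
; SetMirrorMode flips the image through a weighted post-process material on the first PostProcessVolume found.
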(event `self.ReceiveBeginPlay`
  ;[1 1 1] Create UI
  (bind _returnvalue (`|CreateWidget` "/Game/WebcamController/UI/W_WebCamSelectorUI.W_WebCamSelectorUI_C" (`GameplayStatics.GetPlayerController` 0)))
  (`UserWidget.AddToViewport` _returnvalue 0)
  (set `self.UI` _returnvalue)
  (`self.Start`))

(event `SetMirrorMode`
  (params (bIsMirrored :type Boolean))
  (bind _outactors (`GameplayStatics.GetAllActorsOfClass` "/Script/Engine.PostProcessVolume"))
  (if (> (`KismetArrayLibrary.Array_Length` _outactors) 0)
    (setmembers `PostProcessSettings` :`StructRef` (`PostProcessVolume.Settings` (`|GetArrayItem` _outactors)) :`WeightedBlendables` (make `WeightedBlendables` (`|MakeArray` (make `WeightedBlendable` (`KismetMathLibrary.Conv_BoolToDouble` bIsMirrored) "/Game/WebcamController/Materials/PP_FlipHorizontal.PP_FlipHorizontal") :!type "WeightedBlendable Structure")))))

(event `Start`
  (bind _bt_startbutton (`/Game/WebcamController/UI/W_WebCamSelectorUI.BT_StartButton` (`self.UI`)))
  (`ComboBoxString.ClearOptions` (`/Game/WebcamController/UI/W_WebCamSelectorUI.CB_FrameRates` (`self.UI`)))
  (`ComboBoxString.ClearOptions` (`/Game/WebcamController/UI/W_WebCamSelectorUI.CB_Resolutions` (`self.UI`)))
  (`ComboBoxString.ClearOptions` (`/Game/WebcamController/UI/W_WebCamSelectorUI.CB_TrackNumber` (`self.UI`)))
  (`ComboBoxString.ClearOptions` (`/Game/WebcamController/UI/W_WebCamSelectorUI.CB_WebcamNames` (`self.UI`)))
  (`Widget.SetIsEnabled` _bt_startbutton false)
  (add `Button.OnClicked` _bt_startbutton (delegate `OnStartWebcam`))
  (bind _devices (`self.Update Device Names`))
  (set `self.CameraDevices` _devices)
  (add `ComboBoxString.OnSelectionChanged` (`/Game/WebcamController/UI/W_WebCamSelectorUI.CB_WebcamNames` (`self.UI`)) (delegate `OnWebcamSelected`))
  (`ComboBoxString.SetSelectedIndex` (`/Game/WebcamController/UI/W_WebCamSelectorUI.CB_WebcamNames` (`self.UI`)) 0))

(event `OnWebcamSelected`
  (params (SelectedItem :type String) (SelectionType :type "ESelectInfo Enum" :default "OnKeyPress"))
  (`Widget.SetIsEnabled` (`/Game/WebcamController/UI/W_WebCamSelectorUI.BT_StartButton` (`self.UI`)) false)
  (`KismetSystemLibrary.Delay` 0.2)
  (`ComboBoxString.ClearOptions` (`/Game/WebcamController/UI/W_WebCamSelectorUI.CB_FrameRates` (`self.UI`)))
  (`ComboBoxString.ClearOptions` (`/Game/WebcamController/UI/W_WebCamSelectorUI.CB_Resolutions` (`self.UI`)))
  (`ComboBoxString.ClearOptions` (`/Game/WebcamController/UI/W_WebCamSelectorUI.CB_TrackNumber` (`self.UI`)))
  (bind _capturedevice (`self.Find Capture Device by Name` (`KismetTextLibrary.Conv_StringToText` SelectedItem)))
  (`self.OpenMediaPlayer` (`.Url` (break `MediaCaptureDevice` _capturedevice))))

(event `Stop`
  (`MediaPlayer.Pause` (`self.MediaPlayer`)))

(event `OnStartWebcam`
  (bind _cb_framerates (`/Game/WebcamController/UI/W_WebCamSelectorUI.CB_FrameRates` (`self.UI`)))
  (if (`MediaPlayer.IsPlaying` (`self.MediaPlayer`))
    (`MediaPlayer.Close` (`self.MediaPlayer`))
    (`TextBlock.SetText` (`/Game/WebcamController/UI/W_WebCamSelectorUI.T_ButtonText` (`self.UI`)) "Start")
    (`Widget.SetIsEnabled` _cb_framerates true)
    (`Widget.SetIsEnabled` (`/Game/WebcamController/UI/W_WebCamSelectorUI.CB_Resolutions` (`self.UI`)) true)
    (`Widget.SetIsEnabled` (`/Game/WebcamController/UI/W_WebCamSelectorUI.CB_WebcamNames` (`self.UI`)) true)
    (`self.OnWebcamStopped`)
    (`self.Start`)
    (else
      (bind _returnvalue (`MediaPlayer.Play` (`self.MediaPlayer`)))
      (`KismetSystemLibrary.PrintString` (`KismetStringLibrary.Conv_BoolToString` _returnvalue))
      (`TextBlock.SetText` (`/Game/WebcamController/UI/W_WebCamSelectorUI.T_ButtonText` (`self.UI`)) "Stop")
      (`Widget.SetIsEnabled` _cb_framerates false)
      (`Widget.SetIsEnabled` (`/Game/WebcamController/UI/W_WebCamSelectorUI.CB_Resolutions` (`self.UI`)) false)
      (`Widget.SetIsEnabled` (`/Game/WebcamController/UI/W_WebCamSelectorUI.CB_TrackNumber` (`self.UI`)) false)
      (`Widget.SetIsEnabled` (`/Game/WebcamController/UI/W_WebCamSelectorUI.CB_WebcamNames` (`self.UI`)) false)
      (`self.OnWebcamStarted`))))

(event `OpenMediaPlayer`
  (params (Url :type String))
  (bind _cb_tracknumber (`/Game/WebcamController/UI/W_WebCamSelectorUI.CB_TrackNumber` (`self.UI`)))
  (`MediaPlayer.OpenUrl` (`self.MediaPlayer`) Url)
  (`KismetSystemLibrary.Delay` 0.2)
  (`ComboBoxString.ClearOptions` (`/Game/WebcamController/UI/W_WebCamSelectorUI.CB_TrackNumber` (`self.UI`)))
  (for _index (range (`MediaPlayer.GetNumTracks` (`self.MediaPlayer`) "Video"))
    (`ComboBoxString.AddOption` _cb_tracknumber (`KismetStringLibrary.Conv_IntToString` _index)))
  (add `ComboBoxString.OnSelectionChanged` _cb_tracknumber (delegate `OnTrackSelected`))
  (`ComboBoxString.SetSelectedOption` _cb_tracknumber (`KismetStringLibrary.Conv_IntToString` (- (`MediaPlayer.GetNumTracks` (`self.MediaPlayer`) "Video") 1))))

(event `self.ReceiveEndPlay`
  (params (EndPlayReason :type "EEndPlayReason Enum" :default "Destroyed"))
  (`self.Stop`))

(event `OnTrackSelected`
  (params (SelectedItem :type String) (SelectionType :type "ESelectInfo Enum" :default "OnKeyPress"))
  (set `self.TrackIndex` (`KismetStringLibrary.Conv_StringToInt` SelectedItem))
  (add `ComboBoxString.OnSelectionChanged` (`/Game/WebcamController/UI/W_WebCamSelectorUI.CB_Resolutions` (`self.UI`)) (delegate `OnResolutionChanged`))
  (`self.UpdateResolutions`))

(event `OnResolutionChanged`
  (params (SelectedItem :type String) (SelectionType :type "ESelectInfo Enum" :default "OnKeyPress"))
  (bind (_lefts _rights) (`KismetStringLibrary.Split` SelectedItem "x"))
  (`KismetSystemLibrary.Delay` 0.1)
  (set `self.SelectedResolution` (make `IntPoint` (`KismetStringLibrary.Conv_StringToInt` _lefts) (`KismetStringLibrary.Conv_StringToInt` _rights)))
  (add `ComboBoxString.OnSelectionChanged` (`/Game/WebcamController/UI/W_WebCamSelectorUI.CB_FrameRates` (`self.UI`)) (delegate `OnFrameRateSelected`))
  (`self.UpdateFPS`))

(event `OnFrameRateSelected`
  (params (SelectedItem :type String) (SelectionType :type "ESelectInfo Enum" :default "OnKeyPress"))
  (`KismetSystemLibrary.Delay` 0.1)
  (set `self.SelectedFPS` (`KismetStringLibrary.Conv_StringToDouble` SelectedItem))
  (`MediaPlayer.SelectTrack` (`self.MediaPlayer`) "Video" (`self.TrackIndex`))
  (bind _format (`self.Find Format Index`))
  (set `self.SelectedFormat` _format)
  (`MediaPlayer.SetTrackFormat` (`self.MediaPlayer`) "Video" (`self.TrackIndex`) _format)
  (`KismetSystemLibrary.PrintString` (`KismetStringLibrary.Concat_StrStr` (`KismetStringLibrary.Concat_StrStr` "Format selected: " (`KismetStringLibrary.Conv_IntToString` (`self.SelectedFormat`))) " - " (`KismetStringLibrary.Conv_IntPointToString` (`self.SelectedResolution`)) " - " (`KismetStringLibrary.Conv_DoubleToString` (`self.SelectedFPS`))))
  (`Widget.SetIsEnabled` (`/Game/WebcamController/UI/W_WebCamSelectorUI.CB_TrackNumber` (`self.UI`)) false)
  (`KismetSystemLibrary.Delay` 0.1)
  (`MediaPlayer.Pause` (`self.MediaPlayer`))
  (`KismetSystemLibrary.Delay` 0.5)
  (`Widget.SetIsEnabled` (`/Game/WebcamController/UI/W_WebCamSelectorUI.BT_StartButton` (`self.UI`)) true))

(fn `Find Capture Device by Name`
  (params (DevieName :type Text))
  (returns (CaptureDevice :type "MediaCaptureDevice Structure"))
  (for _array_element (`self.CameraDevices`)
    (if (`KismetTextLibrary.EqualEqual_TextText` (`.DisplayName` (break `MediaCaptureDevice` _array_element)) DevieName)
      (return _array_element)))
  (`KismetSystemLibrary.PrintString` "Can't find device by name")
  (`KismetSystemLibrary.PrintString` (`KismetTextLibrary.Conv_TextToString` DevieName)))

(fn `Find Format Index`
  (returns (Format :type Integer))
  (bind _trackindex (`self.TrackIndex`))
  (bind _mediaplayer (`self.MediaPlayer`))
  (for _index (range (`MediaPlayer.GetNumTrackFormats` (`self.MediaPlayer`) "Video" (`self.TrackIndex`)))
    (if (and (`KismetMathLibrary.Equal_IntPointIntPoint` (`MediaPlayer.GetVideoTrackDimensions` _mediaplayer _trackindex _index) (`self.SelectedResolution`)) (== (`MediaPlayer.GetVideoTrackFrameRate` _mediaplayer _trackindex _index) (`self.SelectedFPS`)))
      (return _index)))
  (return 0))

(fn `Update Device Names`
  (returns (Devices :type "Array of MediaCaptureDevice Structure"))
  (`ComboBoxString.ClearOptions` (`/Game/WebcamController/UI/W_WebCamSelectorUI.CB_WebcamNames` (`self.UI`)))
  (bind _outdevices (`MediaBlueprintFunctionLibrary.EnumerateVideoCaptureDevices` -1))
  (for _array_element _outdevices
    (`ComboBoxString.AddOption` (`/Game/WebcamController/UI/W_WebCamSelectorUI.CB_WebcamNames` (`self.UI`)) (`KismetTextLibrary.Conv_TextToString` (`.DisplayName` (break `MediaCaptureDevice` _array_element)))))
  (return _outdevices))

(fn `UpdateFPS`
  (locals (AvailableFPS :type "Array of Float (double-precision)") (bFoundPreferedFPS :type Boolean))
  (`KismetArrayLibrary.Array_Clear` (`local.AvailableFPS`))
  (`|ExecutionSequence`
    (:`then_0`
      (`ComboBoxString.ClearOptions` (`/Game/WebcamController/UI/W_WebCamSelectorUI.CB_FrameRates` (`self.UI`))))
    (:`then_1`
      (for _index (range (`MediaPlayer.GetNumTrackFormats` (`self.MediaPlayer`) "Video" (`self.TrackIndex`)))
        (if (`KismetMathLibrary.Equal_IntPointIntPoint` (`MediaPlayer.GetVideoTrackDimensions` (`self.MediaPlayer`) (`self.TrackIndex`) _index) (`self.SelectedResolution`))
          (`KismetArrayLibrary.Array_AddUnique` (`local.AvailableFPS`) (`MediaPlayer.GetVideoTrackFrameRate` (`self.MediaPlayer`) (`self.TrackIndex`) _index))))
      (set `local.bFoundPreferedFPS` false)
      (for (_array_element _array_index) (`local.AvailableFPS`)
        (`ComboBoxString.AddOption` (`/Game/WebcamController/UI/W_WebCamSelectorUI.CB_FrameRates` (`self.UI`)) (`KismetStringLibrary.Conv_DoubleToString` _array_element))
        (if (== (`self.PreferedFPS`) _array_element)
          (`ComboBoxString.SetSelectedIndex` (`/Game/WebcamController/UI/W_WebCamSelectorUI.CB_FrameRates` (`self.UI`)) _array_index)
          (set `local.bFoundPreferedFPS` true)))
      (if (not (`local.bFoundPreferedFPS`))
        (`ComboBoxString.SetSelectedIndex` (`/Game/WebcamController/UI/W_WebCamSelectorUI.CB_FrameRates` (`self.UI`)) 0)))))

(fn `UpdateResolutions`
  (locals (AvailableResolutions :type "Array of Vector2D Structure") (bFoundPrefered :type Boolean))
  (`KismetArrayLibrary.Array_Clear` (`local.AvailableResolutions`))
  (`|ExecutionSequence`
    (:`then_0`
      (`ComboBoxString.ClearOptions` (`/Game/WebcamController/UI/W_WebCamSelectorUI.CB_Resolutions` (`self.UI`))))
    (:`then_1`
      (for _index (range (`MediaPlayer.GetNumTrackFormats` (`self.MediaPlayer`) "Video" (`self.TrackIndex`)))
        (`KismetArrayLibrary.Array_AddUnique` (`local.AvailableResolutions`) (`KismetMathLibrary.Conv_IntPointToVector2D` (`MediaPlayer.GetVideoTrackDimensions` (`self.MediaPlayer`) (`self.TrackIndex`) _index))))
      (set `local.bFoundPrefered` false)
      (for (_array_element _array_index) (`local.AvailableResolutions`)
        (bind (_x _y) (`KismetMathLibrary.BreakVector2D` _array_element))
        (`ComboBoxString.AddOption` (`/Game/WebcamController/UI/W_WebCamSelectorUI.CB_Resolutions` (`self.UI`)) (`KismetStringLibrary.Concat_StrStr` (`KismetStringLibrary.Conv_IntToString` (`KismetMathLibrary.Round` _x)) "x" (`KismetStringLibrary.Conv_IntToString` (`KismetMathLibrary.Round` _y))))
        (if (== _array_element (`self.PreferedResoltution`))
          (`ComboBoxString.SetSelectedIndex` (`/Game/WebcamController/UI/W_WebCamSelectorUI.CB_Resolutions` (`self.UI`)) _array_index)
          (set `local.bFoundPrefered` true)))
      (if (not (`local.bFoundPrefered`))
        (`ComboBoxString.SetSelectedIndex` (`/Game/WebcamController/UI/W_WebCamSelectorUI.CB_Resolutions` (`self.UI`)) 0)))))

(fn `UserConstructionScript`)